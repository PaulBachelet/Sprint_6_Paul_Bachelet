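; BP_Ladder is a climbable ladder prop whose construction script builds frames and rungs to a set Height and sizes the use trigger.
; A FlipFlop, unconnected here, toggles mounting, which interpolates the player onto the trigger and binds forward input, and dismounting.
; Input plays root-motion climb montages in Flying mode for vertical movement.
; A retriggerable delay pauses climbing upon input release; reaching either end restores walking.
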(event `self.ReceiveTick`
  (params (DeltaSeconds :type "Float (single-precision)"))
  (bind _usetrigger (`self.UseTrigger`))
  (`/Engine/EditorBlueprintResources/StandardMacros.Gate` true :!label _label
    (:`Exit`
      (`/Game/DarkRPGTemplate/Blueprints/FunctionLibraries/BP_DarkRPG_FuntionLibrary.InterpActorToLocationAndRotation` (`self.Player`) (`SceneComponent.K2_GetComponentLocation` _usetrigger) (`SceneComponent.K2_GetComponentRotation` _usetrigger) 8.0 true true) ; Move the player to the target location every tick while \nusing the ladder
    )))

(event `OpenInterpGate`
  (goto _label :!via `Open`))

(event `CloseInterpGate`
  (goto _label :!via `Close`))

(event `MoveOnLadder`
  (params (Up :type Boolean))
  (bind _z (.z (`self.K2_GetActorLocation`)))
  (`|ExecutionSequence`
    (:`then_0`
      (`/Engine/EditorBlueprintResources/StandardMacros.DoOnce` false :!label _label_2 ; Stops calling the animation many\ntimes
        (:`Completed`
          (`self.CloseInterpGate`) ; Stop forcing the player to the trigger\nlocation
          (`/Game/DarkRPGTemplate/Blueprints/Player/BP_Player.PlayMontage` (`self.Player`) (select `bool` Up :`false` "/Game/DarkRPGTemplate/Animations/Player/Anim_BaseMale_LadderClimbDown_Montage.Anim_BaseMale_LadderClimbDown_Montage" :`true` "/Game/DarkRPGTemplate/Animations/Player/Anim_BaseMale_LadderClimb_Montage.Anim_BaseMale_LadderClimb_Montage" :!type "AnimMontage Object Reference")) ; Montage has root motion to move\nthe player up
          (`CharacterMovementComponent.SetMovementMode` (`Character.CharacterMovement` (`self.Player`)) "MOVE_Flying" 0) ; But Z axis root motion only works\nin flying movement mode
        )))
    (:`then_1`
      (if (not (`KismetMathLibrary.NearlyEqual_FloatFloat` (.z (`self.K2_GetActorLocation` (`self.Player`))) (+ (select `bool` Up :`false` _z :`true` (+ _z (* (`KismetMathLibrary.Conv_IntToDouble` (`self.Height`)) 50.0))) 100.0) 10.0))
        (`KismetSystemLibrary.RetriggerableDelay` 0.1) ; Won't let execution through unless \nthe player lets go of movement input
        (`/Engine/EditorBlueprintResources/StandardMacros.Gate` true :!label _label_3 ; Stops execution if we get to the\ntop/bottom of the ladder
          (:`Exit`
            (`AnimInstance.Montage_Pause` (`SkeletalMeshComponent.GetAnimInstance` (`Character.Mesh` (`self.Player`))) (select `bool` Up :`false` "/Game/DarkRPGTemplate/Animations/Player/Anim_BaseMale_LadderClimbDown_Montage.Anim_BaseMale_LadderClimbDown_Montage" :`true` "/Game/DarkRPGTemplate/Animations/Player/Anim_BaseMale_LadderClimb_Montage.Anim_BaseMale_LadderClimb_Montage" :!type "AnimMontage Object Reference")) ; Pause the ladder animation\nwhere it is
            (`MovementComponent.StopMovementImmediately` (`Character.CharacterMovement` (`self.Player`))) ; Stops the player gliding upwards\nbecause of momentum
            (`/Game/DarkRPGTemplate/Blueprints/Interfaces/BP_PawnInteraction_Interface.ActorCanMove` (`self.Player`) false) ; Ensures the player can't move around\nwhile stopped on the ladder
            (`self.ResetMoveInput`) ; Resets move input so we can\nstart climbing again
          ))
        (else
          (`self.FinishedLadder`) ; Otherwise come off the ladder
        )))))

(event `ResetMoveInput`
  (goto _label_2 :!via `Reset`))

(event `LadderMounted`
  (goto _label_3 :!via `Open`))

(event `LadderDismounted`
  (goto _label_3 :!via `Close`))

(event `FinishedLadder`
  (bind _player (`self.Player`))
  (`CharacterMovementComponent.SetMovementMode` (`Character.CharacterMovement` (`self.Player`)) "MOVE_Walking" 0) ; Return the movement mode to walking
  (`self.CloseInterpGate`) ; Make sure player is not\ngetting forced to the trigger\nlocation
  (`/Game/DarkRPGTemplate/Blueprints/Interfaces/BP_PawnInteraction_Interface.ActorCanMove` _player true) ; Allow the player to move freely\nagain
  (clear `/Game/DarkRPGTemplate/Blueprints/Player/BP_Player.MoveForwardPressed` _player) ; Unbind the ladder move forward event\nfrom player's input
  (`Character.StopAnimMontage` (`self.Player`) null) ; Stop the ladder montage
  (`self.LadderDismounted`) ; Prevent the ladder from\nthinking we've only stopped\non the ladder
  (`self.ResetMoveInput`) ; Resets move input so when\nmounted again we can climb
)

(fn `UserConstructionScript`
  (locals (CurrentHeight :type "Float (double-precision)"))
  (for _ (range 1 (+ (`self.Height`) 1))
    (`AddComponent|NODE_AddStaticMeshComponent-0` :`RelativeTransform` (`KismetMathLibrary.MakeTransform` (`KismetMathLibrary.MakeVector` 0.0 0.0 (`local.CurrentHeight`)))) ; Add a new ladder frame
    (`AddComponent|NODE_AddStaticMeshComponent-1` :`RelativeTransform` (`KismetMathLibrary.MakeTransform` (`KismetMathLibrary.MakeVector` 0.0 0.0 (+ (`local.CurrentHeight`) 20.0)))) ; Add a new ladder rung
    (set `local.CurrentHeight` (+ (`local.CurrentHeight`) 50.0)) ; Increase the height by 50
  )
  (`BoxComponent.SetBoxExtent` (`self.UseTrigger`) (`KismetMathLibrary.MakeVector` 48.0 50.0 (* (`self.Height`) 50.0)) true) ; Set the height of the use trigger\nso it can be used at the bottom and\ntop of the ladder
)